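; GravTestDynamic is a test actor that simulates switchable gravity on its static mesh through keyboard input.
; It enables input for player 0 on BeginPlay, then adds GravVelocity to the mesh's physics linear velocity every Tick, unscaled by delta time.
; The I, K, J, L, U and O keys aim that vector along the world axes, and releasing any of them resets it to downward.
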(event `self.ReceiveBeginPlay`
  (`self.EnableInput` (`GameplayStatics.GetPlayerController` 0)))

(event `self.ReceiveTick`
  (params (DeltaSeconds :type "Float (single-precision)"))
  (`PrimitiveComponent.SetPhysicsLinearVelocity` (`self.StaticMeshComponent`) (`self.GravVelocity`) true "None"))

(event `Key|I`
  (params (Key :type "Key Structure"))
  (:`Pressed`
    (set `self.GravVelocity` (0.0 0.0 9.8)))
  (:`Released`
    (set `self.GravVelocity` (0.0 0.0 -9.8) :!label _label)))

(event `Key|K`
  (params (Key :type "Key Structure"))
  (:`Pressed`
    (goto _label))
  (:`Released`
    (goto _label)))

(event `Key|J`
  (params (Key :type "Key Structure"))
  (:`Pressed`
    (set `self.GravVelocity` (0.0 -9.8 0.0)))
  (:`Released`
    (goto _label)))

(event `Key|L`
  (params (Key :type "Key Structure"))
  (:`Pressed`
    (set `self.GravVelocity` (0.0 9.8 0.0)))
  (:`Released`
    (goto _label)))

(event `Key|U`
  (params (Key :type "Key Structure"))
  (:`Pressed`
    (set `self.GravVelocity` (9.8 0.0 0.0)))
  (:`Released`
    (goto _label)))

(event `Key|O`
  (params (Key :type "Key Structure"))
  (:`Pressed`
    (set `self.GravVelocity` (-9.8 0.0 0.0)))
  (:`Released`
    (goto _label)))

(fn `UserConstructionScript`)