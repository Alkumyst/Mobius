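; GravParentC is an actor Blueprint that simulates mutual gravitational attraction between all instances of its class.
; Every Tick it gathers all GravParentC actors and adds velocity to its own physics mesh toward each one.
; The pull is a fixed constant over squared distance, with no mass or delta-time scaling.
; The loop does not exclude the actor itself.
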(event `self.ReceiveTick`
  (params (DeltaSeconds :type "Float (single-precision)"))
  (bind _returnvalue (`self.K2_GetActorLocation`))
  (bind _outactors (`GameplayStatics.GetAllActorsOfClass` "GravParentC_C"))
  (for _array_element _outactors
    (bind _returnvalue_2 (`self.K2_GetActorLocation` _array_element))
    (`PrimitiveComponent.SetPhysicsLinearVelocity` (`self.StaticMeshComponent`) (* (`KismetMathLibrary.GetForwardVector` (`KismetMathLibrary.FindLookAtRotation` _returnvalue _returnvalue_2)) (/ 400000.0 (`KismetMathLibrary.VSizeSquared` (- _returnvalue_2 _returnvalue)))) true "None")))

(fn `UserConstructionScript`)