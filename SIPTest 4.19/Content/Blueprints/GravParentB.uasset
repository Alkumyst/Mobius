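; GravParentB is a parent actor Blueprint that makes its instances pull toward one another like simple mutual gravity.
; Each Tick it gathers every other GravParentB and adds a fixed-magnitude velocity to its own physics StaticMesh, aimed at each one's mesh.
; The pull ignores distance, mass and delta time, so it is frame-rate dependent and rescans all instances every frame.
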(event `self.ReceiveTick`
  (params (DeltaSeconds :type "Float (single-precision)"))
  (bind _outactors (`GameplayStatics.GetAllActorsOfClass` "GravParentB_C"))
  (for _array_element _outactors
    (if (not (== _array_element self))
      (bind _asgrav_parent_type_2 (cast `/Game/Blueprints/GravParentB` _array_element))
      (`PrimitiveComponent.SetPhysicsLinearVelocity` (`self.StaticMesh`) (* (`KismetMathLibrary.GetForwardVector` (`KismetMathLibrary.FindLookAtRotation` (`SceneComponent.K2_GetComponentLocation` (`self.StaticMesh`)) (`SceneComponent.K2_GetComponentLocation` (`/Game/Blueprints/GravParentB.StaticMesh` _asgrav_parent_type_2)))) 9.8) true "None"))))

(fn `UserConstructionScript`)