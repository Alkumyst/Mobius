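; GravParentA is a parent-named actor that simulates mutual gravitational attraction between its instances using physics.
; Every tick it gathers all GravParentA actors and, for each one other than itself, adds linear velocity to its StaticMesh toward that actor.
; The pull follows an inverse-square falloff with a hardcoded strength, independent of mass and not scaled by delta time.
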(event `self.ReceiveTick`
  (params (DeltaSeconds :type "Float (single-precision)"))
  (bind _returnvalue (`SceneComponent.K2_GetComponentLocation` (`self.StaticMesh`)))
  (bind _outactors (`GameplayStatics.GetAllActorsOfClass` "GravParentA_C"))
  (for _array_element _outactors
    (if (not (== _array_element self))
      (bind _returnvalue_2 (`self.K2_GetActorLocation` _array_element))
      (`PrimitiveComponent.SetPhysicsLinearVelocity` (`self.StaticMesh`) (* (`KismetMathLibrary.GetForwardVector` (`KismetMathLibrary.FindLookAtRotation` _returnvalue _returnvalue_2)) (/ 400000.0 (`KismetMathLibrary.VSizeSquared` (- _returnvalue_2 _returnvalue)))) true "None"))))

(fn `UserConstructionScript`)